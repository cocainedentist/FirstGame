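; BP_Arrow is a physics-driven arrow projectile that damages the characters it hits and destroys itself after a short lifetime.
; An impulse on BeginPlay launches its Sphere forward, and Tick rotates it along its velocity while it simulates physics.
; A blocking hit stops the simulation.
; Overlapping a Character mid-flight also stops it, attaches it to that character's mesh and adds damage through BP_PlayerState.
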(event `self.ReceiveBeginPlay`
  (bind _sphere (`self.Sphere`))
  (`PrimitiveComponent.AddImpulse` _sphere (* (`SceneComponent.GetForwardVector` _sphere) 5000.0) "None" false)
  (`KismetSystemLibrary.Delay` 5.0)
  (`self.K2_DestroyActor`))

(event `self.ReceiveTick`
  (params (DeltaSeconds :type "Float (single-precision)"))
  (bind _sphere (`self.Sphere`))
  (if (`SceneComponent.IsSimulatingPhysics` (`self.Sphere`) "None")
    (bind _returnvalue (`PrimitiveComponent.GetPhysicsLinearVelocity` _sphere "None"))
    (`SceneComponent.K2_SetWorldRotation` _sphere (`KismetMathLibrary.MakeRotFromX` _returnvalue) false false)))

(event `self.Sphere.OnComponentHit`
  (params (HitComponent :type "PrimitiveComponent Object Reference") (OtherActor :type "Actor Object Reference") (OtherComp :type "PrimitiveComponent Object Reference") (NormalImpulse :type "Vector Structure") (Hit :type "HitResult Structure (by ref)"))
  (`PrimitiveComponent.SetSimulatePhysics` (`self.Sphere`) false))

(event `self.Sphere.OnComponentBeginOverlap`
  (params (OverlappedComponent :type "PrimitiveComponent Object Reference") (OtherActor :type "Actor Object Reference") (OtherComp :type "PrimitiveComponent Object Reference") (OtherBodyIndex :type Integer) (bFromSweep :type Boolean) (SweepResult :type "HitResult Structure (by ref)"))
  (if (`SceneComponent.IsSimulatingPhysics` (`self.Sphere`) "None")
    (bind _ascharacter (cast `Character` OtherActor))
    (`PrimitiveComponent.SetSimulatePhysics` (`self.Sphere`) false)
    (`self.K2_AttachToComponent` (`Character.Mesh` _ascharacter) "None" "KeepWorld" "KeepWorld" "KeepWorld")
    (bind _asbp_player_state (cast `/Game/ThirdPerson/Blueprints/BP_PlayerState` (`Pawn.PlayerState` _ascharacter)))
    (`/Game/ThirdPerson/Blueprints/BP_PlayerState.AddDamage` _asbp_player_state 5.0)))

(fn `UserConstructionScript`)