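; BP_ArrowCannon is a cannon that fires BP_Arrow projectiles in a scattered spread.
; On BeginPlay it calls ToggleCannon, then sets LoopTime to a short interval; neither the toggle nor the loop logic is defined here.
; ShootCannon spawns each arrow at the Arrow component's location, aimed in a random direction within a narrow cone around that component's forward vector.
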(event `self.ReceiveBeginPlay`
  (`self.ToggleCannon`)
  (set `self.LoopTime` 0.1))

(fn `ShootCannon`
  (bind (_returnvalue_location _returnvalue_rotation) (`KismetMathLibrary.BreakTransform` (`SceneComponent.K2_GetComponentToWorld` (`self.Arrow`))))
  (`|SpawnActorFromClass` "/Game/FirstGame/Blueprints/Projectiles/BP_Arrow.BP_Arrow_C" (`KismetMathLibrary.MakeTransform` _returnvalue_location (`KismetMathLibrary.MakeRotFromX` (`KismetMathLibrary.RandomUnitVectorInConeInDegrees` (`KismetMathLibrary.GetForwardVector` _returnvalue_rotation) 10.0))) "Undefined" "MultiplyWithRoot" null null))

(fn `UserConstructionScript`
  (`parent.UserConstructionScript`))