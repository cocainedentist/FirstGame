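; Cannon variant with limited ammo that fires one shot per ToggleCannon event.
; BeginPlay loads ten shots, and the ShootCannon override calls the parent's shot, decrements the count and updates the CountWidget, printing a warning once empty.
; Every tick it turns the widget toward the player camera using only X and Y, so the counter stays upright.
; The parent's BeginPlay and Tick are not called.
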(event `self.ToggleCannon`
  (`self.ShootCannon`))

(event `self.ReceiveBeginPlay`
  (set `self.Count` 10)
  (bind _ascount_widget (cast `/Game/FirstGame/Widgets/CountWidget` (`WidgetComponent.GetUserWidgetObject` (`self.Widget`))))
  (`/Game/FirstGame/Widgets/CountWidget.SetCount` _ascount_widget (`self.Count`)))

(event `self.ReceiveTick`
  (params (DeltaSeconds :type "Float (single-precision)"))
  (`self.UpdateLookCamera`))

(fn `ShootCannon`
  (if (> (`self.Count`) 0)
    (`parent.ShootCannon`)
    (set `self.Count` (- (`self.Count`) 1))
    (bind _ascount_widget (cast `/Game/FirstGame/Widgets/CountWidget` (`WidgetComponent.GetUserWidgetObject` (`self.Widget`))))
    (`/Game/FirstGame/Widgets/CountWidget.SetCount` _ascount_widget (`self.Count`))
    (else
      (`KismetSystemLibrary.PrintString` "OUT OF AMMO!!"))))

(fn `UpdateLookCamera`
  (bind (_returnvalue_x _returnvalue_y) (`KismetMathLibrary.BreakVector` (`self.K2_GetActorLocation` (`GameplayStatics.GetPlayerCameraManager` 0))))
  (bind (_returnvalue_x_2 _returnvalue_y_2) (`KismetMathLibrary.BreakVector` (`SceneComponent.K2_GetComponentLocation` (`self.Widget`))))
  (`SceneComponent.K2_SetWorldRotation` (`self.Widget`) (`KismetMathLibrary.FindLookAtRotation` (`KismetMathLibrary.MakeVector` _returnvalue_x_2 _returnvalue_y_2) (`KismetMathLibrary.MakeVector` _returnvalue_x _returnvalue_y)) false false))

(fn `UserConstructionScript`
  (`parent.UserConstructionScript`))